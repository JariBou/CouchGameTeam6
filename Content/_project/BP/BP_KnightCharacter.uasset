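; Player character Blueprint for a team-based game where each character is either a Knight or a Squire.
; On start it binds gameplay sound triggers to per-type sounds played at its location, then registers with the HUD's health widget a tick later.
; A ragdoll-arms event mixes physical animation with selective bone simulation.
; Each tick it passes team and type to a debug text widget.
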(event `PlayDeathSound`
  (`self.PlaySounds` (`/Game/_project/Data/Blueprints_DataSounds/BPDA_KnightSounds.Death` (`self.KnightSoundsData`)) (`/Game/_project/Data/Blueprints_DataSounds/BPDA_SquireSounds.Death` (`self.SquireSoundsData`))))

(event `PlayDropSound`
  (`self.PlaySounds` (`/Game/_project/Data/Blueprints_DataSounds/BPDA_KnightSounds.Drop` (`self.KnightSoundsData`)) (`/Game/_project/Data/Blueprints_DataSounds/BPDA_SquireSounds.Drop` (`self.SquireSoundsData`))))

(event `PlayDodgeSound`
  (`self.PlaySounds` (`/Game/_project/Data/Blueprints_DataSounds/BPDA_KnightSounds.Dodge` (`self.KnightSoundsData`)) (`/Game/_project/Data/Blueprints_DataSounds/BPDA_SquireSounds.Dash` (`self.SquireSoundsData`))))

(event `PlayMoveSound`
  (`self.PlaySounds` (`/Game/_project/Data/Blueprints_DataSounds/BPDA_KnightSounds.Move` (`self.KnightSoundsData`)) (`/Game/_project/Data/Blueprints_DataSounds/BPDA_SquireSounds.Move` (`self.SquireSoundsData`))))

(event `PlayPickupSound`
  (`self.PlaySounds` null (`/Game/_project/Data/Blueprints_DataSounds/BPDA_SquireSounds.Pickup` (`self.SquireSoundsData`))))

(event `PlayTakeDamageSound`
  (`self.PlaySounds` (`/Game/_project/Data/Blueprints_DataSounds/BPDA_KnightSounds.HitTaken` (`self.KnightSoundsData`)) (`/Game/_project/Data/Blueprints_DataSounds/BPDA_SquireSounds.HitTaken` (`self.SquireSoundsData`))))

(event `PlayRespawnSound`
  (`self.PlaySounds` (`/Game/_project/Data/Blueprints_DataSounds/BPDA_KnightSounds.Respawn` (`self.KnightSoundsData`)) (`/Game/_project/Data/Blueprints_DataSounds/BPDA_SquireSounds.Respawn` (`self.SquireSoundsData`))))

(event `self.ReceiveBeginPlay`
  (add `self.TriggerRespawnSound` (delegate `PlayRespawnSound`))
  (add `self.TriggerDropSound` (delegate `PlayDropSound`))
  (add `self.TriggerDeathSound` (delegate `PlayDeathSound`))
  (add `self.TriggerDodgeSound` (delegate `PlayDodgeSound`))
  (add `self.TriggerMoveSound` (delegate `PlayMoveSound`))
  (add `self.TriggerPickupSound` (delegate `PlayPickupSound`))
  (add `self.TriggerTakeDamageSound` (delegate `PlayTakeDamageSound`))
  (`KismetSystemLibrary.DelayUntilNextTick`)
  (bind _asbp_hud_game (cast `/Game/_project/BP/BP_HudGame` (`PlayerController.GetHUD` (`GameplayStatics.GetPlayerController` 0))))
  (`/Game/_project/Widgets/W_InGame.BindCharacterToHealthEvent` (`/Game/_project/BP/BP_HudGame.InGameWidget` _asbp_hud_game) self))

(event `self.ActivateRagdollArms`
  (bind _mesh (`self.Mesh`))
  (`PhysicalAnimationComponent.SetSkeletalMeshComponent` (`self.PhysicalAnimation`) (`self.Mesh`))
  (`PhysicalAnimationComponent.ApplyPhysicalAnimationSettingsBelow` (`self.PhysicalAnimation`) (`self.BoneForArmsRagdoll`) (make `PhysicalAnimationData` true 100000.0 100.0 1000.0 100.0 1000.0 1000.0) true)
  (`SkeletalMeshComponent.SetAllBodiesBelowSimulatePhysics` _mesh (`self.BoneForArmsRagdoll`) false false)
  (`SkeletalMeshComponent.SetAllBodiesBelowSimulatePhysics` _mesh (`self.BoneHand`) true true)
  (`SkeletalMeshComponent.SetAllBodiesBelowSimulatePhysics` _mesh (`self.In Bone Name`) true true))

(event `self.ReceiveTick`
  (params (DeltaSeconds :type "Float (single-precision)"))
  (bind _aswd_player_debug_text (cast `/Game/_project/Widgets/Debug/WD_PlayerDEbugText` (`WidgetComponent.GetWidget` (`self.Widget`))))
  (`/Game/_project/Widgets/Debug/WD_PlayerDEbugText.CE_PassText` _aswd_player_debug_text (`KismetTextLibrary.Conv_NameToText` (`|GetEnumeratorName` (`self.PlayerTeam`))) (`KismetTextLibrary.Conv_NameToText` (`|GetEnumeratorName` (`self.PlayerType`)))))

(fn `PlaySounds`
  (params (KnightSound :type "SoundBase Object Reference") (SquireSound :type "SoundBase Object Reference"))
  (bind _returnvalue (`self.K2_GetActorLocation`))
  (switch `TypeOfPlayer` (`self.PlayerType`)
    (:`Knight`
      (`GameplayStatics.PlaySoundAtLocation` KnightSound _returnvalue (struct) 1.0 1.0 0.0 null null null null))
    (:`Squire`
      (`GameplayStatics.PlaySoundAtLocation` SquireSound _returnvalue (struct) 1.0 1.0 0.0 null null null null))))

(fn `UserConstructionScript`)