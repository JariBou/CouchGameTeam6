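; BP_KillZone is an environment trigger volume that kills characters and destroys pickables entering it.
; When an actor overlaps its Box, a living SfCharacter is killed, and otherwise a Pickable is destroyed through DestroyPickable.
; The construction script sizes the Box from the BoxSize variable.
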(event `self.Box.OnComponentBeginOverlap`
  (params (OverlappedComponent :type "PrimitiveComponent Object Reference") (OtherActor :type "Actor Object Reference") (OtherComp :type "PrimitiveComponent Object Reference") (OtherBodyIndex :type Integer) (bFromSweep :type Boolean) (SweepResult :type "HitResult Structure (by ref)"))
  (bind _assf_character (cast `SfCharacter` OtherActor)
    (:`then`
      (if (not (`SfCharacter.IsDead` _assf_character))
        (`SfCharacter.Kill` _assf_character null)))
    (:`CastFailed`
      (bind _aspickable (cast `Pickable` OtherActor))
      (`Pickable.DestroyPickable` _aspickable))))

(fn `UserConstructionScript`
  (`BoxComponent.SetBoxExtent` (`self.Box`) (`self.BoxSize`) true))