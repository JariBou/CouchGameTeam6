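; Game HUD Blueprint that owns the in-game UI and provides helpers for spawning and switching widgets.
; On BeginPlay it creates and displays W_InGame only when the owning player's controller ID is 0.
; CreateWidget builds a given widget class inside that widget's InnerCanvas and returns it.
; ChangeMenuWidget swaps one menu for a new one on player 0's viewport, storing the removed menu's class as LastMenu.
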(event `self.ReceiveBeginPlay`
  (bind _playerowner (`self.PlayerOwner`))
  (if (== (`GameplayStatics.GetPlayerControllerID` _playerowner) 0)
    (bind _returnvalue (`|CreateWidget` "/Game/_project/Widgets/W_InGame.W_InGame_C" _playerowner))
    (bind _output_get (set `self.InGameWidget` _returnvalue))
    (`UserWidget.AddToViewport` _output_get 0)))

(fn `ChangeMenuWidget`
  (params (`New Menu` :type "UserWidget Class Reference") (MenuToRemove :type "UserWidget Object Reference"))
  (`Widget.RemoveFromParent` MenuToRemove)
  (bind _returnvalue (`|CreateWidget` `New Menu` (`GameplayStatics.GetPlayerController` 0)))
  (`UserWidget.AddToViewport` _returnvalue 0)
  (set `self.LastMenu` (`GameplayStatics.GetObjectClass` MenuToRemove)))

(fn `CreateWidget`
  (params (WidgetToCreate :type "UserWidget Class Reference"))
  (returns (CreatedWidget :type "UserWidget Object Reference"))
  (bind _returnvalue (`|CreateWidget` WidgetToCreate (`self.PlayerOwner`)))
  (`CanvasPanel.AddChildToCanvas` (`/Game/_project/Widgets/W_InGame.InnerCanvas` (`self.InGameWidget`)) _returnvalue)
  (return _returnvalue))

(fn `UserConstructionScript`)