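; Consumable spawner Blueprint that shows a floating indicator while a spawned consumable is waiting to be picked up.
; Spawn and pickup events toggle a visibility flag; the spawning logic itself is not in this graph.
; While visible, Tick bobs the indicator above its BeginPlay location with an absolute-sine Lerp, resetting the phase when hidden.
; Every tick also rotates the indicator to face the main camera from CameraWorldSubsystem, billboard-style.
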(event `self.ReceiveBeginPlay`
  (set `self.First Transform` (`KismetMathLibrary.MakeTransform` (`SceneComponent.K2_GetComponentLocation` (`self.Indicator`)))))

(event `self.ReceiveTick`
  (params (DeltaSeconds :type "Float (single-precision)"))
  (bind _first_transform (`self.First Transform`))
  (bind _indicator (`self.Indicator`))
  (bind _indicator_2 (`self.Indicator`))
  (bind (_returnvalue_x _returnvalue_y _returnvalue_z) (`KismetMathLibrary.BreakVector` (+ (`KismetMathLibrary.MakeVector` (.x (.location _first_transform)) (.y (.location _first_transform)) (.z (.location _first_transform))) (0.0 0.0 40.0))))
  (`|ExecutionSequence`
    (:`then_0`
      (if (`self.ShouldIndicatorBeVisible`)
        (`|ExecutionSequence`
          (:`then_0`
            (`SceneComponent.SetVisibility` (`self.Indicator`) true false))
          (:`then_1`
            (bind _output_get (set `self.ArrowAugment` (+ (`self.ArrowAugment`) (* DeltaSeconds (`self.Speed`)))))
            (`SceneComponent.K2_SetWorldTransform` _indicator (`KismetMathLibrary.MakeTransform` (`KismetMathLibrary.MakeVector` (.x (.location _first_transform)) (.y (.location _first_transform)) (`KismetMathLibrary.Lerp` (.z (.location _first_transform)) _returnvalue_z (`KismetMathLibrary.Abs` (`KismetMathLibrary.Sin` _output_get)))) (`SceneComponent.K2_GetComponentRotation` _indicator)) true false)))
        (else
          (set `self.ArrowAugment` 0.0)
          (`SceneComponent.SetVisibility` (`self.Indicator`) false false))))
    (:`then_1`
      (`SceneComponent.K2_SetWorldRotation` _indicator_2 (`KismetMathLibrary.FindLookAtRotation` (`SceneComponent.K2_GetComponentLocation` _indicator_2) (`SceneComponent.K2_GetComponentLocation` (`CameraWorldSubsystem.CameraMain` (subsystem `CameraWorldSubsystem`)))) false false))))

(event `self.OnConsumableSpawned`
  (set `self.ShouldIndicatorBeVisible` true))

(event `self.OnConsumablePickedUp`
  (set `self.ShouldIndicatorBeVisible` false))

(fn `UserConstructionScript`)