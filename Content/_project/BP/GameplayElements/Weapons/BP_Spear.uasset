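; Spear weapon Blueprint that damages characters its damage box overlaps, apart from its own holder.
; On overlap, it casts the other actor to SfCharacter, checks that it can be damaged, then applies custom damage credited to the holder.
; A successful hit plays the weapon hit sound at the spear's location and calls DealtDamage.
; An IsValid check on the holder exists but is unconnected.
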(event `self.DmgBox.OnComponentBeginOverlap`
  (params (OverlappedComponent :type "PrimitiveComponent Object Reference") (OtherActor :type "Actor Object Reference") (OtherComp :type "PrimitiveComponent Object Reference") (OtherBodyIndex :type Integer) (bFromSweep :type Boolean) (SweepResult :type "HitResult Structure (by ref)"))
  (bind _holder (`self.Holder`))
  (if (not (== OtherActor _holder))
    (bind _assf_character (cast `SfCharacter` OtherActor))
    (bind _returnvalue (`SfCharacter.CanBeDamagedCustom` _assf_character))
    (if _returnvalue
      (bind _returnvalue_2 (`SfCharacter.TakeDamageCustom` _assf_character _holder (`self.GetDamage`)))
      (if _returnvalue_2
        (`GameplayStatics.PlaySoundAtLocation` (`self.WeaponHitSound`) (`self.K2_GetActorLocation`) (struct) 1.0 1.0 0.0 null null null null)
        (`self.DealtDamage`)))))

(fn `UserConstructionScript`
  (`parent.UserConstructionScript`))