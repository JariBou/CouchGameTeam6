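; BP_Well is a well gameplay element with an Indicator component that bobs up and down as a marker.
; The construction script caches the Indicator's starting world location.
; While ArrowIsVisible is set, Tick advances a speed-scaled timer, feeding an absolute sine into a lerp that bounces the Indicator up to 100 units above that point.
; When the flag is off, only the timer resets.
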(event `self.ReceiveTick`
  (params (DeltaSeconds :type "Float (single-precision)"))
  (bind _first_transform (`self.First Transform`))
  (bind _indicator (`self.Indicator`))
  (bind (_returnvalue_x _returnvalue_y _returnvalue_z) (`KismetMathLibrary.BreakVector` (+ (`KismetMathLibrary.MakeVector` (.x (.location _first_transform)) (.y (.location _first_transform)) (.z (.location _first_transform))) (0.0 0.0 100.0))))
  (if (`self.ArrowIsVisible`)
    (bind _output_get (set `self.ArrowAugment` (+ (`self.ArrowAugment`) (* DeltaSeconds (`self.Speed`)))))
    (`SceneComponent.K2_SetWorldTransform` _indicator (`KismetMathLibrary.MakeTransform` (`KismetMathLibrary.MakeVector` (.x (.location _first_transform)) (.y (.location _first_transform)) (`KismetMathLibrary.Lerp` (.z (.location _first_transform)) _returnvalue_z (`KismetMathLibrary.Abs` (`KismetMathLibrary.Sin` _output_get)))) (`SceneComponent.K2_GetComponentRotation` _indicator)) true false)
    (else
      (set `self.ArrowAugment` 0.0))))

(fn `UserConstructionScript`
  (set `self.First Transform` (`KismetMathLibrary.MakeTransform` (`SceneComponent.K2_GetComponentLocation` (`self.Indicator`)))))