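; BP_HudGame is the game HUD Blueprint that manages the pause screen, menu navigation and widgets added to the in-game canvas.
; SetPause opens W_PauseScreen, focuses Resume, adds the menu input mapping and zeroes time dilation through the game mode.
; LastMenu stacks widget classes, so BackInMenu recreates the previous menu.
; The setup that creates W_InGame and caches the game mode is unconnected and never runs.
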(event `self.ReceiveBeginPlay`)

(fn `BackInMenu`
  (bind _lastmenu (`self.LastMenu`))
  (bind _lastmenu_2 (`self.LastMenu`))
  (`Widget.RemoveFromParent` (`self.CurrentMenu`))
  (`KismetArrayLibrary.Array_Remove` _lastmenu_2 (`KismetArrayLibrary.Array_LastIndex` _lastmenu_2))
  (bind _returnvalue (`|CreateWidget` (`|GetArrayItem` _lastmenu (`KismetArrayLibrary.Array_LastIndex` _lastmenu)) (`self.PlayerOwner`)))
  (bind _output_get (set `self.CurrentMenu` _returnvalue))
  (`/Engine/EditorBlueprintResources/StandardMacros.IsValid` _output_get
    (:`Is Valid`
      (`UserWidget.AddToViewport` _output_get 0))))

(fn `ChangeMenuWidget`
  (params (`New Menu` :type "UserWidget Class Reference") (MenuToRemove :type "UserWidget Object Reference"))
  (`Widget.RemoveFromParent` MenuToRemove)
  (bind _returnvalue (`|CreateWidget` `New Menu` (`GameplayStatics.GetPlayerController` 0)))
  (bind _output_get (set `self.CurrentMenu` _returnvalue))
  (`UserWidget.AddToViewport` _output_get 0)
  (`KismetArrayLibrary.Array_Add` (`self.LastMenu`) (`GameplayStatics.GetObjectClass` _returnvalue)))

(fn `CreateWidget`
  (params (WidgetToCreate :type "UserWidget Class Reference"))
  (returns (CreatedWidget :type "UserWidget Object Reference"))
  (bind _returnvalue (`|CreateWidget` WidgetToCreate (`self.PlayerOwner`)))
  (`CanvasPanel.AddChildToCanvas` (`/Game/_project/Widgets/W_InGame.InnerCanvas` (`self.InGameWidget`)) _returnvalue)
  (return _returnvalue))

(fn `SetPause`
  (params (PlayerController :type "PlayerController Object Reference"))
  (locals (PlayerControllerLocal :type "PlayerController Object Reference"))
  (set `local.PlayerControllerLocal` PlayerController)
  (bind _returnvalue (`|CreateWidget` "/Game/_project/Widgets/Menu/Pause_Screen/W_PauseScreen.W_PauseScreen_C" (`local.PlayerControllerLocal`)))
  (set `/Game/_project/Widgets/Menu/Pause_Screen/W_PauseScreen.PlayerController` (`local.PlayerControllerLocal`) _returnvalue)
  (bind _output_get (set `self.CurrentMenu` _returnvalue))
  (`UserWidget.AddToViewport` _output_get 0)
  (`WidgetBlueprintLibrary.SetInputMode_GameAndUIEx` (`local.PlayerControllerLocal`) (`/Game/_project/Widgets/Menu/Pause_Screen/W_PauseScreen.Button_Resume` _returnvalue))
  (`KismetArrayLibrary.Array_Add` (`self.LastMenu`) (`GameplayStatics.GetObjectClass` _returnvalue))
  (message `EnhancedInputSubsystemInterface.AddMappingContext` (pcsubsystem `EnhancedInputLocalPlayerSubsystem` (`local.PlayerControllerLocal`)) "/Game/_project/Input/IMC_InMenus.IMC_InMenus" 0 (struct))
  (`SfGameMode.SetTimeDilation` (`self.BP Sf Game Mode`) 0.0))

(fn `UserConstructionScript`)