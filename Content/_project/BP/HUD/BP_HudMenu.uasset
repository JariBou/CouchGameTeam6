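; Menu HUD that opens the start screen for the first player and manages navigation between menu widgets.
; A stack of widget classes in LastMenu records each opened menu, so Back recreates the previous one rather than keeping instances alive.
; It binds to BP_ControllerMenu's back and confirm dispatchers.
; It also forwards controller navigation to the team selection widget and passes P1 confirm when the game can start.
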(event `self.ReceiveBeginPlay`
  (bind _returnvalue (`GameplayStatics.GetPlayerController` 0))
  (bind _playerowner (`self.PlayerOwner`))
  (if (== (`GameplayStatics.GetPlayerControllerID` _playerowner) 0)
    (bind _returnvalue_2 (`|CreateWidget` "/Game/_project/Widgets/Menu/Start_Screen/W_StartScreen.W_StartScreen_C" _playerowner))
    (`UserWidget.AddToViewport` _returnvalue_2 0)
    (`KismetArrayLibrary.Array_Add` (`self.LastMenu`) (`GameplayStatics.GetObjectClass` _returnvalue_2))
    (`WidgetBlueprintLibrary.SetInputMode_UIOnlyEx` _returnvalue (`/Game/_project/Widgets/Menu/Start_Screen/W_StartScreen.Button_Play` _returnvalue_2))
    (set `PlayerController.bShowMouseCursor` true _returnvalue)
    (bind _asbp_controller_menu (cast `/Game/_project/BP/BP_ControllerMenu` _returnvalue))
    (add `/Game/_project/BP/BP_ControllerMenu.ED_Back` _asbp_controller_menu (delegate `GoBackInMenu`))
    (add `/Game/_project/BP/BP_ControllerMenu.ED_Confirm` _asbp_controller_menu (`|CreateDelegate` :!event `OnP1Confirm`))))

(event `GoBackInMenu`
  (bind _lastmenu (`self.LastMenu`))
  (bind _lastmenu_2 (`self.LastMenu`))
  (if (> (`KismetArrayLibrary.Array_Length` (`self.LastMenu`)) 1)
    (`Widget.RemoveFromParent` (`self.CurrentMenu`))
    (`KismetArrayLibrary.Array_Remove` _lastmenu_2 (`KismetArrayLibrary.Array_LastIndex` _lastmenu_2))
    (bind _returnvalue (`|CreateWidget` (`|GetArrayItem` _lastmenu (`KismetArrayLibrary.Array_LastIndex` _lastmenu)) (`self.PlayerOwner`)))
    (bind _output_get (set `self.CurrentMenu` _returnvalue))
    (`UserWidget.AddToViewport` _output_get 0)))

(event `ControllerNavigateInput`
  (params (Controller :type "/Game/_project/BP/BP_ControllerMenu Object Reference") (Direction :type "Float (double-precision)"))
  (if (!= (`self.TeamSelectionWidget`) null)
    (`/Game/_project/Widgets/Menu/Team_selection/W_TeamSelectionMenu.LinkControllerToMovePlayerWidget` (`self.TeamSelectionWidget`) Direction (`GameplayStatics.GetPlayerControllerID` Controller))))

(event `OnP1Confirm`
  (bind _teamselectionwidget (`self.TeamSelectionWidget`))
  (`/Engine/EditorBlueprintResources/StandardMacros.IsValid` _teamselectionwidget
    (:`Is Valid`
      (bind _state (`/Game/_project/Widgets/Menu/Team_selection/W_TeamSelectionMenu.Can Game be Started` _teamselectionwidget))
      (if _state
        (`/Game/_project/Widgets/Menu/Team_selection/W_TeamSelectionMenu.OnP1Confirm` _teamselectionwidget)))))

(fn `ChangeMenuWidget`
  (params (NewMenu :type "UserWidget Class Reference") (MenuToRemove :type "UserWidget Object Reference"))
  (`Widget.RemoveFromParent` MenuToRemove)
  (bind _returnvalue (`|CreateWidget` NewMenu (`GameplayStatics.GetPlayerController` 0)))
  (bind _output_get (set `self.CurrentMenu` _returnvalue))
  (`UserWidget.AddToViewport` _output_get 0)
  (`KismetArrayLibrary.Array_Add` (`self.LastMenu`) (`GameplayStatics.GetObjectClass` _returnvalue)))

(fn `CreateWidget`
  (params (WidgetToCreate :type "UserWidget Class Reference"))
  (returns (WidgetCreated :type "UserWidget Object Reference"))
  (bind _returnvalue (`|CreateWidget` WidgetToCreate (`self.PlayerOwner`)))
  (`UserWidget.AddToViewport` _returnvalue 0)
  (return _returnvalue))

(fn `UserConstructionScript`)