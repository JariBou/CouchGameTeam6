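; BP_HudMenu is a menu HUD Blueprint that shows the start screen and handles switching between menu widgets.
; On BeginPlay it creates W_StartScreen for its owning player and adds it to the viewport.
; ChangeMenuWidget removes the current menu, creates the requested widget class for player controller 0, and records the removed widget's class in LastMenu.
; A controller-ID check for showing the start screen is left disconnected.
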(event `self.ReceiveBeginPlay`
  (bind _returnvalue (`|CreateWidget` "/Game/_project/Widgets/Menu/Start_Screen/W_StartScreen.W_StartScreen_C" (`self.PlayerOwner`)))
  (`UserWidget.AddToViewport` _returnvalue 0))

(fn `ChangeMenuWidget`
  (params (NewMenu :type "UserWidget Class Reference") (MenuToRemove :type "UserWidget Object Reference"))
  (`Widget.RemoveFromParent` MenuToRemove)
  (bind _returnvalue (`|CreateWidget` NewMenu (`GameplayStatics.GetPlayerController` 0)))
  (`UserWidget.AddToViewport` _returnvalue 0)
  (set `self.LastMenu` (`GameplayStatics.GetObjectClass` MenuToRemove)))

(fn `UserConstructionScript`)